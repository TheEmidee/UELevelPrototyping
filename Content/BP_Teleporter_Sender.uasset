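; Teleporter sender pad that moves any Character overlapping its trigger to the linked Destination's teleport point, keeping the Character's rotation.
; The construction script previews the link by reading the Destination's name, color and plate scale to set the label, tint the plate and pointer, and size the plate.
; It also yaws the actor to face the Destination and labels an unlinked pad as having no destination.
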(event `self.Trigger.OnComponentBeginOverlap`
  (params (OverlappedComponent :type "PrimitiveComponent Object Reference") (OtherActor :type "Actor Object Reference") (OtherComp :type "PrimitiveComponent Object Reference") (OtherBodyIndex :type Integer) (bFromSweep :type Boolean) (SweepResult :type "HitResult Structure (by ref)"))
  (cast `Character` OtherActor)
  (`self.K2_TeleportTo` OtherActor (`SceneComponent.K2_GetComponentLocation` (`/LevelPrototyping/BP_Teleporter_Destination.TeleportPoint` (`self.Destination`))) (`self.K2_GetActorRotation` OtherActor)))

(fn `UpdateColor`
  (bind _destination (`self.Destination`)
    (:`then`
      (bind _returnvalue (`KismetMathLibrary.Conv_LinearColorToVector` (`/LevelPrototyping/BP_Teleporter_Destination.Color` _destination)))
      (`MeshComponent.SetVectorParameterValueOnMaterials` (`self.Plate`) "Base Color" _returnvalue)
      (`MeshComponent.SetVectorParameterValueOnMaterials` (`self.Pointer`) "Base Color" _returnvalue))
    (:`else`)))

(fn `UpdateName`
  (`self.Destination`
    (:`then`
      (`TextRenderComponent.K2_SetText` (`self.DestinationName`) (`|FormatText` "To \n{Desitnation}" (`/LevelPrototyping/BP_Teleporter_Destination.DestinationName` (`self.Destination`)))))
    (:`else`
      (`TextRenderComponent.K2_SetText` (`self.DestinationName`) "No \nDestination"))))

(fn `UpdateRotation`
  (bind _destination (`self.Destination`)
    (:`then`
      (bind (_returnvalue_roll _returnvalue_pitch _returnvalue_yaw) (`KismetMathLibrary.BreakRotator` (`KismetMathLibrary.FindLookAtRotation` (`self.K2_GetActorLocation`) (`self.K2_GetActorLocation` _destination))))
      (`self.K2_SetActorRotation` (`KismetMathLibrary.MakeRotator` 0.0 0.0 _returnvalue_yaw)))
    (:`else`)))

(fn `UpdateScale`
  (bind _destination (`self.Destination`)
    (:`then`
      (bind _platescale (`/LevelPrototyping/BP_Teleporter_Destination.PlateScale` _destination))
      (`SceneComponent.SetWorldScale3D` (`self.Plate`) (`KismetMathLibrary.MakeVector` _platescale _platescale 0.02)))
    (:`else`)))

(fn `UserConstructionScript`
  (`self.UpdateName`)
  (`self.UpdateColor`)
  (`self.UpdateRotation`)
  (`self.UpdateScale`))